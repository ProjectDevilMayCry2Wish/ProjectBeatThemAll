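; BP_HealthPickup is a collectible that heals the third-person character on sphere overlap.
; It heals by HealAmount through the character's AC_Health component only when health is below full, so it stays in place otherwise.
; An IsConsumed flag guards against repeat use, then the pickup calls sound and emitter spawns, destroys itself and prints a debug string.
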(event `self.Sphere.OnComponentBeginOverlap`
  (params (OverlappedComponent :type "PrimitiveComponent Object Reference") (OtherActor :type "Actor Object Reference") (OtherComp :type "PrimitiveComponent Object Reference") (OtherBodyIndex :type Integer) (bFromSweep :type Boolean) (SweepResult :type "HitResult Structure (by ref)"))
  (if (not (`self.IsConsumed`))
    (bind _asbp_third_person_character (cast `/Game/ThirdPerson/Blueprints/BP_ThirdPersonCharacter` OtherActor))
    (bind _returnvalue (`self.GetComponentByClass` _asbp_third_person_character "/Game/Core/Component/AC_Health.AC_Health_C"))
    (if (< (`/Game/Core/Component/AC_Health.GetHealthPercent` _returnvalue) 1.0)
      (`/Game/Core/Component/AC_Health.Heal` _returnvalue (`self.HealAmount`))
      (set `self.IsConsumed` true)
      ;[1 0.08985 0.6492 0.5] SOUND
      (`GameplayStatics.PlaySoundAtLocation` null (0.0 0.0 0.0) (struct) 1.0 1.0 0.0 null null null null)
      ;[1 0.08985 0.6492 0.5] EFFET
      (`GameplayStatics.SpawnEmitterAtLocation` null)
      (`self.K2_DestroyActor`)
      (`KismetSystemLibrary.PrintString` "Hello"))))

(fn `UserConstructionScript`)