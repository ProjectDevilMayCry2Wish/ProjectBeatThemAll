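; Attack manager that limits how many enemies attack at once through a shared pool of tokens.
; RequestToken grants a slot while under MaxTokens, otherwise queues the enemy in WaitingEnemies.
; ReleaseToken clears the enemy from both lists and calls GrantNextToken, which finds the waiting enemy nearest the player but only stores it in BestEnemy.
; A looping CleanUp timer purges destroyed enemies, re-running that selection when a holder was removed.
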(event `self.ReceiveBeginPlay`
  (`KismetSystemLibrary.K2_SetTimer` null "CleanUp" 1.0 true))

(fn `CleanUp`
  (locals (IsRemovedSomething :type Boolean))
  ;[0 0 0 0.5] Sécurité. Toutes les secondes, retire les ennemis détruits des listes pour qu’ils ne bloquent jamais un token.
  ;;[0.15 0.1452 0.0243 0.5] Nettoie les détenteurs de tokens : un ennemi détruit libère sa place.
  (for (_array_element _array_index) (`self.TokenHolders`)
    (`/Engine/EditorBlueprintResources/StandardMacros.IsValid` _array_element
      (:`Is Not Valid`
        (`KismetArrayLibrary.Array_Remove` (`self.TokenHolders`) _array_index)
        (set `local.IsRemovedSomething` true))))
  ;;[0.15 0.1452 0.0243 0.5] Nettoie la file d’attente : on ne veut pas donner un token à un ennemi détruit.
  (bind (_arrayindex _arrayelement) (`/Engine/EditorBlueprintResources/StandardMacros.ReverseForEachLoop` (`self.WaitingEnemies`))
    (:`LoopBody`
      (`/Engine/EditorBlueprintResources/StandardMacros.IsValid` _arrayelement
        (:`Is Not Valid`
          (`KismetArrayLibrary.Array_Remove` (`self.WaitingEnemies`) _arrayindex))))
    (:`Completed`
      (if (`local.IsRemovedSomething`)
        (`self.GrantNextToken`)))))

(fn `GrantNextToken`
  (locals (BestEnemy :type "Actor Object Reference") (BestDistance :type "Float (double-precision)" :default 999999.0))
  ;[0 0 0 0.5] Commentcette fonction choisit quel ennemi en attente la reçoit : le plus proche du joueur. Elle ne renvoie rien, elle agit directement.
  ;;[0.15 0.1452 0.0243 0.5] Compte les ennemis en attente. Zéro = personne à servir.
  (if (not (== (`KismetArrayLibrary.Array_Length` (`self.WaitingEnemies`)) 0))
    ;;[0.15 0.1452 0.0243 0.5] Compte les tokens utilisés. Si c’est égal ou supérieur au maximum, il n’y a plus de place.
    (if (not (>= (`KismetArrayLibrary.Array_Length` (`self.TokenHolders`)) (`self.MaxTokens`)))
      ;;[0.15 0.1452 0.0243 0.5] Cherche l'ennemi en attente le plus proche, Si oui il le choisit
      (for _array_element (`self.WaitingEnemies`)
        (`/Engine/EditorBlueprintResources/StandardMacros.IsValid` _array_element
          (:`Is Valid`
            (bind _returnvalue (`Actor.GetDistanceTo` _array_element (`GameplayStatics.GetPlayerPawn` 0)))
            (if (< _returnvalue (`local.BestDistance`))
              (set `local.BestDistance` _returnvalue)
              (set `local.BestEnemy` _array_element))))))))

(fn `ReleaseToken`
  (params (Enemy :type "Actor Object Reference"))
  ;[0 0 0 0.5] L’ennemi rend son token : il a fini d’attaquer, il est mort ou il est étourdi.
  ;;[0.15 0.1452 0.0243 0.5] Retire l’ennemi de la liste des détenteurs : la place est libérée.
  (`KismetArrayLibrary.Array_RemoveItem` (`self.TokenHolders`) Enemy)
  ;;[0.15 0.1452 0.0243 0.5] Retire aussi l’ennemi de la file d’attente (s’il était mort en attendant, on ne veut plus qu’il reçoive un token).
  (`KismetArrayLibrary.Array_RemoveItem` (`self.WaitingEnemies`) Enemy)
  ;;[0.15 0.1452 0.0243 0.5] Une place vient de se libérer : on la donne tout de suite au prochain ennemi en attente.
  (`self.GrantNextToken`))

(fn `RequestToken`
  (params (Enemy :type "Actor Object Reference"))
  (returns (Succes :type Boolean))
  ;[0 0 0 0.5] Fonction que l’ennemi appelle pour demander : « Ai-je le droit d’attaquer ? » Reçoit l’ennemi en entrée, renvoie vrai ou faux.
  ;;[0.15 0.1452 0.0243 0.5] Il a déjà un token ? Si oui, on retourne TRUE tout de suite
  (if (`KismetArrayLibrary.Array_Contains` (`self.TokenHolders`) Enemy)
    (return true)
    (else
      ;;[0.15 0.1452 0.0243 0.5] Reste-t-il de la place ? Nombre de tokens utilisés
      (if (< (`KismetArrayLibrary.Array_Length` (`self.TokenHolders`)) (`self.MaxTokens`))
        ;;[0.15 0.1452 0.0243 0.5] on donne le token : on l’ajoute aux détenteurs, on le retire de la file d’attente, on retourne TRUE.
        (`KismetArrayLibrary.Array_Add` (`self.TokenHolders`) Enemy)
        (`KismetArrayLibrary.Array_RemoveItem` (`self.WaitingEnemies`) Enemy)
        (return true)
        (else
          (`KismetArrayLibrary.Array_AddUnique` (`self.WaitingEnemies`) Enemy)
          (return false))))))