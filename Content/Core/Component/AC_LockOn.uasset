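; Lock-on component for a Pawn that turns the controller's rotation smoothly toward a locked target each tick, toggling off if the target becomes invalid.
; ToggleLock sphere-overlaps nearby pawns, keeps those targetable through BPI_Targetable, and picks the one closest to view forward within an angle limit using dot products.
; SwichtTarget selects the nearest candidate by yaw in the requested direction, with a cooldown.
; Target and lock changes fire notifications.
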(event `self.ReceiveBeginPlay`
  (bind _aspawn (cast `Pawn` (`self.GetOwner`)))
  (bind _output_get (set `self.OwnerPawn` _aspawn))
  (set `self.OwnerController` (`Pawn.GetController` _output_get)))

(event `self.ReceiveTick`
  (params (DeltaSeconds :type "Float (single-precision)"))
  (if (`self.IsLockOn`)
    (bind _currenttarget (`self.CurrentTarget`)
      (:`then`
        (bind _ownercontroller (`self.OwnerController`)
          (:`then`
            (`Controller.SetControlRotation` _ownercontroller (`KismetMathLibrary.RInterpTo` (`Controller.GetControlRotation` _ownercontroller) (`KismetMathLibrary.FindLookAtRotation` (`Actor.K2_GetActorLocation` (`self.OwnerPawn`)) (`Actor.K2_GetActorLocation` _currenttarget)) DeltaSeconds (`self.RotationInterpSpeed`))))
          (:`else`)))
      (:`else`
        (`self.ToggleLock`)))))

(event `ResetSwicht`
  (`KismetSystemLibrary.Delay` (`self.SwitchCooldown`))
  (set `self.IscanSwitch` true))

(fn `GetCandidates `
  (returns (Canditates :type "Array of Actor Object Reference"))
  (locals (Result :type "Array of Actor Object Reference"))
  ;[0 0 0 0.5] Liste les ennemis ciblables autour
  (bind _outactors (`KismetSystemLibrary.SphereOverlapActors` (`Actor.K2_GetActorLocation` (`self.OwnerPawn`)) (`self.MaxLockDistance`) (`|MakeArray` "ObjectTypeQuery3" :!type "EObjectTypeQuery Enum") null (`|MakeArray` (`self.OwnerPawn`) :!type "Actor Object Reference")))
  (for _array_element _outactors
    (if (`KismetSystemLibrary.DoesImplementInterface` _array_element "/Game/Core/Interface/BPI_Targetable.BPI_Targetable_C")
      (bind _result (message `/Game/Core/Interface/BPI_Targetable.CanBeTargeted` _array_element))
      (if _result
        (`KismetArrayLibrary.Array_Add` (`local.Result`) _array_element))))
  (return (`local.Result`)))

(fn `PickBestTarget`
  (params (Candidates :type "Array of Actor Object Reference"))
  (returns (BestTarget :type "Actor Object Reference"))
  (locals (BestActor :type "Actor Object Reference") (BestDot :type "Float (double-precision)" :default -1.0) (MinDot :type "Float (double-precision)") (CamForward :type "Vector Structure"))
  ;[0 0 0 0.5] parmi les candidats, garder celui qui est le plus au centre de l’écran, en ignorant ceux qui dépassent MaxLockAngle
  (`KismetSystemLibrary.PrintString` (`KismetSystemLibrary.GetDisplayName` (`local.BestActor`)))
  (bind _ownercontroller (`self.OwnerController`)
    (:`then`
      (set `local.CamForward` (`KismetMathLibrary.GetForwardVector` (`Controller.GetControlRotation` _ownercontroller)))
      (set `local.MinDot` (`KismetMathLibrary.DegCos` (`self.MaxLockAngle`)))
      (for _array_element Candidates
        (`/Engine/EditorBlueprintResources/StandardMacros.IsValid` _array_element
          (:`Is Valid`
            (bind _returnvalue (`KismetMathLibrary.Dot_VectorVector` (`local.CamForward`) (`KismetMathLibrary.GetDirectionUnitVector` (`Actor.K2_GetActorLocation` (`self.OwnerPawn`)) (`Actor.K2_GetActorLocation` _array_element))))
            (if (>= _returnvalue (`local.MinDot`))
              (if (> _returnvalue (`local.BestDot`))
                (set `local.BestDot` _returnvalue)
                (bind _output_get (set `local.BestActor` _array_element)))))))
      (return _output_get))
    (:`else`
      (return null))))

(fn `SwichtTarget`
  (params (Direction :type Integer))
  (locals (RefRotation :type "Rotator Structure") (BestDiff :type "Float (double-precision)" :default 9999.0) (NewTarget :type "Actor Object Reference") (OldTarget :type "Actor Object Reference"))
  (if (`self.IsLockOn`)
    (if (`self.IscanSwitch`)
      (bind _currenttarget (`self.CurrentTarget`)
        (:`then`
          (bind _ownerpawn (`self.OwnerPawn`)
            (:`then`
              (set `local.RefRotation` (`KismetMathLibrary.FindLookAtRotation` (`Actor.K2_GetActorLocation` _ownerpawn) (`Actor.K2_GetActorLocation` _currenttarget)))
              (bind _canditates (`self.GetCandidates `))
              (for _array_element _canditates
                (`/Engine/EditorBlueprintResources/StandardMacros.IsValid` _array_element
                  (:`Is Valid`
                    (bind _returnvalue (* (.yaw (`KismetMathLibrary.NormalizedDeltaRotator` (`KismetMathLibrary.FindLookAtRotation` (`Actor.K2_GetActorLocation` (`self.OwnerPawn`)) (`Actor.K2_GetActorLocation` _array_element)) (`local.RefRotation`))) Direction))
                    (if (> _returnvalue 0.0)
                      (if (< _returnvalue (`local.BestDiff`))
                        (set `local.BestDiff` _returnvalue)
                        (set `local.NewTarget` _array_element))))))
              (bind _newtarget (`local.NewTarget`)
                (:`then`
                  (bind _output_get (set `local.OldTarget` (`self.CurrentTarget`)))
                  (set `self.CurrentTarget` _newtarget)
                  (`self.OnTargetChanged` _output_get _newtarget)
                  (set `self.IscanSwitch` false)
                  (`self.ResetSwicht`))
                (:`else`)))
            (:`else`)))
        (:`else`)))))

(fn `ToggleLock`
  (locals (OldTarget :type "Actor Object Reference"))
  ;[0 0 0 0.5] active le lock sur la meilleure cible, ou le coupe s'il est déjà actif.
  (if (`self.IsLockOn`)
    (bind _output_get (set `local.OldTarget` (`self.CurrentTarget`)))
    (set `self.CurrentTarget` null)
    (set `self.IsLockOn` false)
    (`self.OnTargetChanged` _output_get)
    (`self.OnLockStateChanged` false)
    (else
      (bind _canditates (`self.GetCandidates `))
      (bind _besttarget (`self.PickBestTarget` _canditates))
      (`/Engine/EditorBlueprintResources/StandardMacros.IsValid` _besttarget
        (:`Is Valid`
          (bind _output_get_2 (set `self.CurrentTarget` _besttarget))
          (set `self.IsLockOn` true)
          (`self.OnTargetChanged` null _output_get_2)
          (`self.OnLockStateChanged` true))))))