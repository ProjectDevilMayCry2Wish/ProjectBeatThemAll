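; AC_Health is a health component that tracks current and maximum health, death and invulnerability for its owning actor.
; TakeDamage clamps health and returns whether damage landed, broadcasting hit, health-change and death events, or a blocked event while invulnerable.
; Heal restores clamped health unless dead, and health starts at maximum on BeginPlay.
; Other systems react through these event dispatchers and can query the health percentage or toggle invulnerability.
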(event `self.ReceiveBeginPlay`
  (set `self.CurrentHealth` (`self.MaxHealth`))
  (`self.OnHealthChanged` (`self.CurrentHealth`) (`self.MaxHealth`)))

(fn `GetHealthPercent`
  (returns (Percent :type "Float (double-precision)"))
  (return (`KismetMathLibrary.SafeDivide` (`self.CurrentHealth`) (`self.MaxHealth`))))

(fn `Heal`
  (params (Amount :type "Float (double-precision)"))
  (if (`self.IsDead`)
    (return)
    (else
      (bind _output_get (set `self.CurrentHealth` (`KismetMathLibrary.FClamp` (+ (`self.CurrentHealth`) Amount) 0.0 (`self.MaxHealth`))))
      (`self.OnHealthChanged` _output_get (`self.MaxHealth`)))))

(fn `SetInvulnerable`
  (params (Value :type Boolean))
  (set `self.IsInvulnerable` Value))

(fn `TakeDamage`
  (params (Amount :type "Float (double-precision)") (DamageCauser :type "Actor Object Reference"))
  (returns (WasHit :type Boolean))
  (if (`self.IsDead`)
    (return false)
    (elif (`self.IsInvulnerable`)
      (`self.OnDamageBlocked` DamageCauser)
      (return false)
      (else
        (bind _output_get (set `self.CurrentHealth` (`KismetMathLibrary.FClamp` (- (`self.CurrentHealth`) Amount) 0.0 (`self.MaxHealth`))))
        (`self.OnHealthChanged` _output_get (`self.MaxHealth`))
        (`self.OnHit` Amount DamageCauser)
        (if (<= (`self.CurrentHealth`) 0.0)
          (set `self.IsDead` true)
          (`self.OnDeath` DamageCauser)
          (return true)
          (else
            (return true)))))))